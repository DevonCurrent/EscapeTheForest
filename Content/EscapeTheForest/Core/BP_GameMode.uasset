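; BP_GameMode is the EscapeTheForest game mode, managing the level countdown, score and master volume.
; Timer loops on a one-second Delay until IsWin or zero.
; At zero it deducts a life, respawns BP_PlayerCharacter and restarts, or pauses and shows WBP_DeathScreen when no lives remain.
; Events add points, apply a remaining-time bonus through EndScore, and override Master volume through a base sound mix set at BeginPlay.
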(event Custom|Changevolume_Event
  (params (Volume :type Float%20%28single-precision%29))
  (Variables|Default|SetVolumeNum Volume)
  (Audio|SetSoundMixClassOverride "/Game/EscapeTheForest/Audio/Mix_NewSound.Mix_NewSound" "/Engine/EngineSounds/Master.Master" (Variables|Default|GetVolumeNum) 1.0 1.0 true))

(event Custom|EndScore
  (Variables|Default|SetScore (+ (* (Variables|Default|GetCurrentTime) (Variables|Default|GetEndBonusMultiplier)) (Variables|Default|GetScore))))

(event Custom|Timer
  ;[1 1 1] Countdown timer for levels. When reaching 0, the player will lose a life and the level will reset with the time set to 0
  (if (> (Variables|Default|GetCurrentTime) 0) :!label _label
    (if (not (Variables|Default|GetisWin))
      (Variables|Default|SetCurrentTime (- (Variables|Default|GetCurrentTime) 1))
      (Utilities|FlowControl|Delay 1.0)
      (goto _label))
    (else
      (bind _asbp_player_character (Utilities|Casting|CastToBP_PlayerCharacter (Game|GetPlayerCharacter 0)))
      (if (== (Variables|/Game/EscapeTheForest/Core/BP_PlayerCharacter.BP_PlayerCharacter_C|Getlives _asbp_player_character) 0)
        (Game|SetGamePaused true)
        (bind _returnvalue (UserInterface|CreateWidget "/Game/EscapeTheForest/Core/Widgets/WBP_DeathScreen.WBP_DeathScreen_C"))
        (UserInterface|Viewport|AddtoViewport _returnvalue 0)
        (Variables|/Script/Engine.PlayerController|SetbShowMouseCursor (Game|GetPlayerController 0) true)
        (else
          (bind _asbp_player_character_2 (Utilities|Casting|CastToBP_PlayerCharacter (Game|GetPlayerCharacter 0)))
          (Variables|/Game/EscapeTheForest/Core/BP_PlayerCharacter.BP_PlayerCharacter_C|Setlives _asbp_player_character_2 (- (Variables|/Game/EscapeTheForest/Core/BP_PlayerCharacter.BP_PlayerCharacter_C|Getlives _asbp_player_character_2) 1))
          (bind _asbp_player_character_3 (Utilities|Casting|CastToBP_PlayerCharacter (Game|GetPlayerCharacter 0)))
          (Default|RespawnPlayer _asbp_player_character_3)
          (CallFunction|ResetTimer)
          (CallFunction|Timer))))))

(event Custom|ResetTimer
  (Variables|Default|SetCurrentTime (Variables|Default|GetMaxTime)))

(event Custom|AddScore
  (params (Score :type Integer))
  (Variables|Default|SetScore (+ Score (Variables|Default|GetScore))))

(event EventBeginPlay
  (Class|GameplayStatics|SetBaseSoundMix "/Game/EscapeTheForest/Audio/Mix_NewSound.Mix_NewSound"))

(fn ConstructionScript)