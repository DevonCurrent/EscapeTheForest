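; BP_Bat is a flipbook-animated bat enemy that flies along a spline, damaging and knocking back the player on hit.
; A looping timeline, with play rate set by TimelineSpeed, moves it along the FlySpline of a referenced track actor from start to end.
; Tick reapplies the flying flipbook and flips actor rotation according to the direction of X movement, alongside the timeline's spline-based rotation.
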(event Custom|UpdateBatAnimation
  (Sprite|SetFlipbook (Variables|Default|GetSprite) "/Game/EscapeTheForest/Characters/EnemySprites/PFB_BatFlyingAnimation.PFB_BatFlyingAnimation"))

(event EventTick
  (params (DeltaSeconds :type Float%20%28single-precision%29))
  (CallFunction|UpdateBatAnimation)
  (if (> (.x (Transformation|GetWorldLocation (Variables|Collision|GetCapsuleComponent))) (Variables|Default|GetLastXPosition))
    (Transformation|SetActorRotation "0, 0, 0")
    (else
      (Transformation|SetActorRotation "0,180.000000, 0")))
  (Variables|Default|SetLastXPosition (.x (Transformation|GetWorldLocation (Variables|Collision|GetCapsuleComponent)))))

(event EventBeginPlay
  ;[1 1 1] Handles movement of bat along a spline
  (Components|Timeline|SetPlayRate (Variables|Default|GetFlyingBat) (/ 1.0 (Variables|Default|GetTimelineSpeed)))
  (bind _newtrack_0 (Timeline|FlyingBat PlayFromStart)
    (:Update
      (Variables|Default|SetAlpha _newtrack_0)
      (Transformation|SetActorLocationAndRotation (Spline|GetLocationatDistanceAlongSpline (Variables|/Game/EscapeTheForest/Core/EnemyAI/BP_BatSpline.BP_BatSpline_C|GetFlySpline (Variables|Default|GetTrackRef)) (Math|Float|Lerp 0.0 (Spline|GetSplineLength (Variables|/Game/EscapeTheForest/Core/EnemyAI/BP_BatSpline.BP_BatSpline_C|GetFlySpline (Variables|Default|GetTrackRef))) (Variables|Default|GetAlpha)) "World") (Spline|GetRotationatDistanceAlongSpline (Variables|/Game/EscapeTheForest/Core/EnemyAI/BP_BatSpline.BP_BatSpline_C|GetFlySpline (Variables|Default|GetTrackRef)) (Math|Float|Lerp 0.0 (Spline|GetSplineLength (Variables|/Game/EscapeTheForest/Core/EnemyAI/BP_BatSpline.BP_BatSpline_C|GetFlySpline (Variables|Default|GetTrackRef))) (Variables|Default|GetAlpha)) "World")))
    (:Finished
      (Timeline|FlyingBat PlayFromStart))))

(event Collision|EventHit
  (params (MyComp :type Primitive%20Component%20Object%20Reference) (Other :type Actor%20Object%20Reference) (OtherComp :type Primitive%20Component%20Object%20Reference) (bSelfMoved :type Boolean) (HitLocation :type Vector :default "0, 0, 0") (HitNormal :type Vector :default "0, 0, 0") (NormalImpulse :type Vector :default "0, 0, 0") (Hit :type Hit%20Result%20Structure%20%28by%20ref%29))
  ;[1 1 1] If the bat hits the player, hurt the player and knock them back
  (bind _asbp_player_character (Utilities|Casting|CastToBP_PlayerCharacter (Game|GetPlayerCharacter 0)))
  (if (== _asbp_player_character Other)
    (Game|Damage|ApplyDamage _asbp_player_character 1.0 0 0)
    (Default|BounceBack _asbp_player_character (.x (Transformation|GetWorldLocation (Variables|Default|GetSprite))))))

(fn ConstructionScript)