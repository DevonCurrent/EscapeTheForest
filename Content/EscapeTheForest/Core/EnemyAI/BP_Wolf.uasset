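; BP_Wolf is a Paper2D enemy that patrols back and forth and attacks the player on contact.
; A timeline drives horizontal velocity, then pauses, reverses direction and uses a FlipFlop to rotate the wolf before restarting.
; Hitting the player applies damage, triggers its BounceBack and flags an attack.
; Tick selects the attack, walk or idle flipbook from that flag and velocity, clearing the flag after the attack animation's length.
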(event Custom|UpdateWolfAnimation
  (if (Variables|Default|GetBisAttacking)
    (Sprite|SetFlipbook (Variables|Default|GetSprite) "/Game/EscapeTheForest/Characters/EnemySprites/PFB_WolfAttackAnimation.PFB_WolfAttackAnimation")
    (Utilities|FlowControl|Delay (Class|PaperFlipbookComponent|GetFlipbookLength (Variables|Default|GetWolfAttackAnimation)))
    (Variables|Default|SetBisAttacking false)
    (else
      (Sprite|SetFlipbook (Variables|Default|GetSprite) (select (> (Math|Vector|VectorLength (Transformation|GetVelocity)) 0.0) "/Game/EscapeTheForest/Characters/EnemySprites/PFB_WolfWalkAnimation.PFB_WolfWalkAnimation" "/Game/EscapeTheForest/Characters/EnemySprites/PFB_WolfIdleAnimation.PFB_WolfIdleAnimation")))))

(event EventBeginPlay
  (Timeline|WolfMovementTime PlayFromStart
    (:Update
      (Variables|/Script/Engine.MovementComponent|SetVelocity (Variables|Character|GetCharacterMovement) (Math|Vector|MakeVector (Variables|Default|GetwolfVelocity) 0.0 0.0)))
    (:Finished
      (Utilities|FlowControl|Delay 0.0001)
      (Variables|/Script/Engine.MovementComponent|SetVelocity (Variables|Character|GetCharacterMovement) "0, 0, 0")
      (Variables|Default|SetwolfVelocity (* (Variables|Default|GetwolfVelocity) -1.0))
      (Variables|Default|SetBisMovingRight (not (Variables|Default|GetBisMovingRight)))
      (Utilities|FlowControl|Delay 5.0)
      (Utilities|FlowControl|FlipFlop
        (:A
          (Transformation|SetActorRotation "0, 0, 0")
          (Timeline|WolfMovementTime PlayFromStart))
        (:B
          (Transformation|SetActorRotation "0,180.000000, 0")
          (Timeline|WolfMovementTime PlayFromStart))))))

(event EventTick
  (params (DeltaSeconds :type Float%20%28single-precision%29))
  (CallFunction|UpdateWolfAnimation))

(event Collision|EventHit
  (params (MyComp :type Primitive%20Component%20Object%20Reference) (Other :type Actor%20Object%20Reference) (OtherComp :type Primitive%20Component%20Object%20Reference) (bSelfMoved :type Boolean) (HitLocation :type Vector :default "0, 0, 0") (HitNormal :type Vector :default "0, 0, 0") (NormalImpulse :type Vector :default "0, 0, 0") (Hit :type Hit%20Result%20Structure%20%28by%20ref%29))
  (bind _asbp_player_character (Utilities|Casting|CastToBP_PlayerCharacter (Game|GetPlayerCharacter 0)))
  (if (== _asbp_player_character Other)
    (Game|Damage|ApplyDamage _asbp_player_character 1.0 0 0)
    (Default|BounceBack _asbp_player_character (.x (Transformation|GetWorldLocation (Variables|Default|GetSprite))))
    (Variables|Default|SetBisAttacking true)))

(fn ConstructionScript)