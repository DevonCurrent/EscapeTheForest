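; BP_WinLocation is the goal trigger in EscapeTheForest that ends the game in a win when the player character overlaps its box.
; On overlap it disables player input, sets the character's animation number, plays a fanfare and sets IsWin on BP_GameMode.
; After a short delay it calls EndScore on the game mode, shows WBP_WinScreen and reveals the mouse cursor.
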(event OnComponentBeginOverlap(Box)
  (params (OverlappedComponent :type Primitive%20Component%20Object%20Reference) (OtherActor :type Actor%20Object%20Reference) (OtherComp :type Primitive%20Component%20Object%20Reference) (OtherBodyIndex :type Integer) (bFromSweep :type Boolean) (SweepResult :type Hit%20Result%20Structure%20%28by%20ref%29))
  (if (== OtherActor (Game|GetPlayerCharacter 0))
    (bind _asbp_player_character (Utilities|Casting|CastToBP_PlayerCharacter (Game|GetPlayerCharacter 0)))
    (Input|DisableInput _asbp_player_character (Game|GetPlayerController 0))
    (Variables|/Game/EscapeTheForest/Core/BP_PlayerCharacter.BP_PlayerCharacter_C|SetanimationNum _asbp_player_character 2)
    (Audio|PlaySound2D "/Game/EscapeTheForest/Audio/A_TadaFanfare.A_TadaFanfare" 1.0 1.0 0.0 0 0)
    (bind _asbp_game_mode (Utilities|Casting|CastToBP_GameMode (Game|GetGameMode)))
    (Variables|/Game/EscapeTheForest/Core/BP_GameMode.BP_GameMode_C|SetisWin _asbp_game_mode true)
    (Utilities|FlowControl|Delay 3.0)
    (bind _asbp_game_mode_2 (Utilities|Casting|CastToBP_GameMode (Game|GetGameMode)))
    (Default|EndScore _asbp_game_mode_2)
    (bind _returnvalue (UserInterface|CreateWidget "/Game/EscapeTheForest/Core/Widgets/WBP_WinScreen.WBP_WinScreen_C"))
    (UserInterface|Viewport|AddtoViewport _returnvalue 0)
    (Variables|/Script/Engine.PlayerController|SetbShowMouseCursor (Game|GetPlayerController 0) true)))

(event EventBeginPlay)

(event Collision|EventActorBeginOverlap
  (params (OtherActor :type Actor%20Object%20Reference)))

(event EventTick
  (params (DeltaSeconds :type Float%20%28single-precision%29)))

(fn ConstructionScript)