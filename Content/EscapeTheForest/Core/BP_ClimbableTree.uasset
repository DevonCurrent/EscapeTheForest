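; BP_ClimbableTree is a tree actor that lets the player climb while inside its LadderVolume2 overlap volume.
; Overlap begin and end toggle the actor's input and the IsLadder flag for the player.
; Holding Climb calls BP_PlayerCharacter's ClimbUpward repeatedly through a short Delay polling loop.
; Releasing Climb, or the loop finding IsLadder false, restores Walking movement and sets the character's AnimationNum.
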(event OnComponentBeginOverlap(LadderVolume2)
  (params (OverlappedComponent :type Primitive%20Component%20Object%20Reference) (OtherActor :type Actor%20Object%20Reference) (OtherComp :type Primitive%20Component%20Object%20Reference) (OtherBodyIndex :type Integer) (bFromSweep :type Boolean) (SweepResult :type Hit%20Result%20Structure%20%28by%20ref%29))
  (if (== OtherActor (Game|GetPlayerCharacter 0))
    (Input|EnableInput (Game|GetPlayerController 0))
    (Variables|Default|SetIsLadder true)))

(event OnComponentEndOverlap(LadderVolume2)
  (params (OverlappedComponent :type Primitive%20Component%20Object%20Reference) (OtherActor :type Actor%20Object%20Reference) (OtherComp :type Primitive%20Component%20Object%20Reference) (OtherBodyIndex :type Integer))
  (if (== OtherActor (Game|GetPlayerCharacter 0))
    (Input|DisableInput (Game|GetPlayerController 0))
    (Variables|Default|SetIsLadder false)))

(event Input|ActionEvents|InputActionClimb
  (params (Key :type Key%20Structure))
  (bind _returnvalue (Game|GetPlayerCharacter 0))
  (:Pressed
    (if (Variables|Default|GetIsLadder) :!label _label
      (if (Game|Player|IsInputKeyDown (Game|GetPlayerController 0) Key)
        (bind _asbp_player_character (Utilities|Casting|CastToBP_PlayerCharacter _returnvalue))
        (Default|ClimbUpward _asbp_player_character)
        (Utilities|FlowControl|Delay 0.1)
        (goto _label))
      (else
        (Pawn|Components|CharacterMovement|SetMovementMode (Variables|/Script/Engine.Character|GetCharacterMovement (Game|GetPlayerCharacter 0)) "MOVE_Walking" 0 :!label _label_2)
        (bind _asbp_player_character_2 (Utilities|Casting|CastToBP_PlayerCharacter _returnvalue))
        (Variables|/Game/EscapeTheForest/Core/BP_PlayerCharacter.BP_PlayerCharacter_C|SetanimationNum _asbp_player_character_2 4))))
  (:Released
    (goto _label_2)))

(fn ConstructionScript)